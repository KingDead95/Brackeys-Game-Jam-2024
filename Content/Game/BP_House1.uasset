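; BP_House1 is a house actor that picks a random static mesh when play begins.
; BeginPlay sets the House component's mesh from the Houses array using a random index from zero to the array length inclusive, which can land out of bounds.
; It then prints an index and mesh name from separate random rolls, so the debug text may not match the displayed mesh.
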(event EventBeginPlay
  (bind _houses (Variables|Default|GetHouses))
  (bind _houses_2 (Variables|Default|GetHouses))
  (bind _returnvalue (Utilities|Array|Length _houses))
  (bind _returnvalue_2 (Math|Random|RandomIntegerinRange 0 _returnvalue))
  (bind _output (Utilities|Array|Get(acopy) _houses_2 _returnvalue_2))
  (Components|StaticMesh|SetStaticMesh (Variables|Default|GetHouse) _output)
  (Development|PrintString (Utilities|String|Append (Utilities|String|ToString(Integer) _returnvalue_2) "  " (Utilities|GetDisplayName _output))))

(fn ConstructionScript)