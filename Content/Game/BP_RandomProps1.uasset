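; BP_RandomProps1 is a prop actor that randomizes the static mesh on its Prop component at BeginPlay.
; It validates a random index into the Props array, then draws a separate random index to pick the mesh, falling back to SM_Crate_2 when the check fails.
; Both draws range up to the array length inclusive, so the index actually used can fall out of bounds.
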(event EventBeginPlay
  (bind _props (Variables|Default|GetProps))
  (bind _returnvalue (Utilities|Array|Length _props))
  (bind _returnvalue_2 (Math|Random|RandomIntegerinRange 0 _returnvalue))
  (if (Utilities|Array|IsValidIndex (Variables|Default|GetProps) _returnvalue_2)
    (Components|StaticMesh|SetStaticMesh (Variables|Default|GetProp) (Utilities|Array|Get(acopy) (Variables|Default|GetProps) _returnvalue_2))
    (else
      (Components|StaticMesh|SetStaticMesh (Variables|Default|GetProp) "/Game/Arte/Low_Poly_Town/Models/Props/SM_Crate_2.SM_Crate_2"))))

(fn ConstructionScript)