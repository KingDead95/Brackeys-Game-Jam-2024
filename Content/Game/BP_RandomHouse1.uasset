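; BP_RandomHouse1 is a house actor that gives its House mesh component a random look when play begins.
; It tests a random index against the Houses array, then sets a mesh from that array or falls back to SM_House_1.
; The check and the lookup roll separately with an inclusive upper bound of the array length, so the lookup can still land out of range.
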(event EventBeginPlay
  (bind _houses (Variables|Default|GetHouses))
  (bind _returnvalue (Utilities|Array|Length _houses))
  (bind _returnvalue_2 (Math|Random|RandomIntegerinRange 0 _returnvalue))
  (if (Utilities|Array|IsValidIndex (Variables|Default|GetHouses) _returnvalue_2)
    (Components|StaticMesh|SetStaticMesh (Variables|Default|GetHouse) (Utilities|Array|Get(acopy) (Variables|Default|GetHouses) _returnvalue_2))
    (else
      (Components|StaticMesh|SetStaticMesh (Variables|Default|GetHouse) "/Game/Arte/Low_Poly_Town/Models/House/SM_House_1.SM_House_1"))))

(fn ConstructionScript)