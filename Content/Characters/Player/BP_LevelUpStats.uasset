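; Stat upgrade pickup that raises the player's max life or damage by an Amount when touched.
; The Life and Damge flags select the stat and, on BeginPlay, the Niagara effect, with Life taking visual priority.
; Sphere overlap by a Player-tagged actor sends update messages to player state 0 for each set flag, then destroys the pickup after a short delay.
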(event OnComponentBeginOverlap(Sphere)
  (params (OverlappedComponent :type Primitive%20Component%20Object%20Reference) (OtherActor :type Actor%20Object%20Reference) (OtherComp :type Primitive%20Component%20Object%20Reference) (OtherBodyIndex :type Integer) (bFromSweep :type Boolean) (SweepResult :type Hit%20Result%20Structure%20%28by%20ref%29))
  (bind _amount (Variables|Default|GetAmount))
  (if (Actor|ActorHasTag OtherActor "Player")
    (Utilities|FlowControl|Sequence
      (:then_0
        (if (Variables|Default|GetLife)
          (Class|BIStats|UpdateMaxLife(Message) (Game|GetPlayerState 0) _amount)
          (Utilities|FlowControl|Delay 0.2 :!label _label)
          (Actor|DestroyActor)))
      (:then_1
        (if (Variables|Default|GetDamge)
          (Class|BIStats|UpdateDamage(Message) (Game|GetPlayerState 0) _amount)
          (goto _label))))))

(event EventBeginPlay
  (if (Variables|Default|GetLife)
    (Class|NiagaraComponent|SetAsset (Variables|Default|GetNiagara) "/Game/Arte/sA_Megapack_v1/sA_PickupSet_1/Fx/NiagaraSystems/NS_Pickup_3.NS_Pickup_3" true)
    (elif (Variables|Default|GetDamge)
      (Class|NiagaraComponent|SetAsset (Variables|Default|GetNiagara) "/Game/Arte/sA_Megapack_v1/sA_PickupSet_1/Fx/NiagaraSystems/NS_Pickup_2.NS_Pickup_2" true))))

(fn ConstructionScript)